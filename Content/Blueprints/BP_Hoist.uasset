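; BP_Hoist is a spline-riding hoist with front and rear bogeys, spreader bars and a muck box.
; Each tick it places bogeys by distance from the root bogey or from spreader attach points, then aims the spreader bars and hoist and stretches a connector tube between them.
; The construction script caches the front-back bogey's offset.
; UnloadMuckbox stops movement, computes a vertically offset drop location and flags lowering; its physics-detach code is unwired.
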(event EventBeginPlay)

(event EventTick
  (params (DeltaSeconds :type Float%20%28single-precision%29))
  (Utilities|FlowControl|Sequence
    (:then_0
      (Class|Train|UpdateBogeyPosition (Variables|Default|GetRootBogey) 0.0))
    (:then_1
      (Class|Hoist|SetBogeyonSpline (Variables|Default|GetRearBogeyFrontAttachPointSpreader) (Variables|Default|GetRearBogeyFront)))
    (:then_2
      (Class|Train|UpdateBogeyPosition (Variables|Default|GetFrontBogeyBack) (Variables|Default|GetFrontBogeyBackDistanceFromRootBogey)))
    (:then_3
      (Class|Hoist|SetBogeyonSpline (Variables|Default|GetFrontBogeyAttachPointSpreader) (Variables|Default|GetFrontBogeyFront)))
    (:then_4
      (Class|Hoist|RotateSpreaderBar (Variables|Default|GetSpreaderBarRear) (Variables|Default|GetRearBogeyFrontAttachPointBogey))
      (Class|Hoist|RotateSpreaderBar (Variables|Default|GetSpreaderBarFront) (Variables|Default|GetFrontBogeyAttachPointBogey))
      (Class|Hoist|RotateSpreaderBar (Variables|Default|GetHoist) (Variables|Default|GetSpreaderBarFrontAttachPoint)))
    (:then_5
      (Class|Hoist|RotateandScaleConnectorTube (Variables|Default|GetSM_ConnectorTube) (Variables|Default|GetRearConnectorMiddle) (Variables|Default|GetFrontConnectorMiddle)))))

(fn ConstructionScript
  (Variables|Default|SetFrontBogeyBackDistanceFromRootBogey (.x (Variables|/Script/Engine.SceneComponent|GetRelativeLocation (Variables|Default|GetFrontBogeyBack)))))

(fn UnloadMuckbox
  (Variables|Default|SetIsMoving false)
  (bind _output_get (Variables|Default|SetStoppedLocation (Transformation|GetWorldTransform (Variables|Default|GetSM_MuckBox))))
  (Variables|Default|SetDropLocation (Math|Transform|MakeTransform (Math|Vector|MakeVector (.x (.location _output_get)) (.y (.location _output_get)) (- (.z (.location _output_get)) -2e+02)) (.rotation _output_get) "1.000000,1.000000,1.000000"))
  (Variables|Default|SetIsLowering true))